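; Actor that manages a capped pool of footstep and grunt sound slots for ants.
; Add and Remove claim or free slots, starting or stopping footsteps, while AddFootstep and AddGrunt register the sound components.
; Tick moves occupied slots' sounds to their ants and triggers short grunts from random start offsets.
; Each slot's grunt interval and duration are randomized once at BeginPlay.
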(event EventBeginPlay
  (while (< (Variables|Default|Geti) (Variables|Default|GetMAX_SOUNDING))
    (Utilities|Array|SetArrayElem (Variables|Default|Getsa_grunt_wait) (Variables|Default|Geti) (+ (* (Math|Random|RandomFloat) 12.0) 1.0))
    (bind _returnvalue (Actor|GetActorOfClass "/Game/Blueprints/BP_AntAI.BP_AntAI_C"))
    (Utilities|Array|Add (Variables|Default|Getsounding_ants) _returnvalue)
    (Utilities|Array|SetArrayElem (Variables|Default|Getsa_grunt_play_time) (Variables|Default|Geti) (+ (* (Math|Random|RandomFloat) 0.3) 0.1))
    (Variables|Default|Seti (+ (Variables|Default|Geti) 1))))

(event EventTick
  (params (DeltaSeconds :type Float%20%28single-precision%29))
  (bind _sa_grunt_wait_ctr (Variables|Default|Getsa_grunt_wait_ctr))
  (for (_array_element _array_index) (Variables|Default|Getsa_empty)
    (if (not _array_element)
      (Transformation|SetWorldLocation (Utilities|Array|Get(acopy) (Variables|Default|Getsa_footsteps) _array_index) (Transformation|GetActorLocation (Utilities|Array|Get(acopy) (Variables|Default|Getsounding_ants) _array_index)) false false)
      (if (Utilities|Array|Get(acopy) (Variables|Default|Getsa_playing_grunt) _array_index)
        (Transformation|SetWorldLocation (Utilities|Array|Get(acopy) (Variables|Default|Getsa_grunts) _array_index) (Transformation|GetActorLocation (Utilities|Array|Get(acopy) (Variables|Default|Getsounding_ants) _array_index)) false false)
        (if (>= (+ (Utilities|Array|Get(acopy) (Variables|Default|Getsa_grunt_wait_ctr) _array_index) DeltaSeconds) (Utilities|Array|Get(acopy) (Variables|Default|Getsa_grunt_play_time) _array_index))
          (Utilities|Array|SetArrayElem (Variables|Default|Getsa_playing_grunt) _array_index false)
          (Utilities|Array|SetArrayElem (Variables|Default|Getsa_grunt_wait_ctr) _array_index 0.0))
        (else
          (Utilities|Array|SetArrayElem _sa_grunt_wait_ctr _array_index (+ (Utilities|Array|Get(acopy) _sa_grunt_wait_ctr _array_index) DeltaSeconds))
          (if (>= (+ (Utilities|Array|Get(acopy) _sa_grunt_wait_ctr _array_index) DeltaSeconds) (Utilities|Array|Get(acopy) (Variables|Default|Getsa_grunt_wait) _array_index))
            (Transformation|SetWorldLocation (Utilities|Array|Get(acopy) (Variables|Default|Getsa_grunts) _array_index) (Transformation|GetActorLocation (Utilities|Array|Get(acopy) (Variables|Default|Getsounding_ants) _array_index)) false false)
            (Audio|Components|Audio|Play (Utilities|Array|Get(acopy) (Variables|Default|Getsa_grunts) _array_index) (* (Math|Random|RandomFloat) (Variables|Default|Getsa_grunt_start_range)))
            (Utilities|Array|SetArrayElem (Variables|Default|Getsa_playing_grunt) _array_index true)
            (Utilities|Array|SetArrayElem (Variables|Default|Getsa_grunt_wait_ctr) _array_index 0.0)
            (Audio|Components|Audio|StopDelayed (Utilities|Array|Get(acopy) (Variables|Default|Getsa_grunts) _array_index) (Utilities|Array|Get(acopy) (Variables|Default|Getsa_grunt_play_time) _array_index))))))))

(fn Add
  (params (ant :type BP%20Ant%20AI%20Object%20Reference))
  (if (< (Variables|Default|Getassigned_ct) (Variables|Default|GetMAX_SOUNDING))
    (Variables|Default|Setalready_stored false)
    (bind _array_element (Utilities|Array|ForEachLoopwithBreak (Variables|Default|Getsounding_ants) :!label _label)
      (:LoopBody
        (if (== _array_element ant)
          (Variables|Default|Setalready_stored true)
          (goto _label Break)))
      (:Completed
        (if (not (Variables|Default|Getalready_stored))
          (Math|Integer|IncrementInt (Variables|Default|Getassigned_ct)
            (:%20%20
              (bind (_array_element_2 _array_index) (Utilities|Array|ForEachLoopwithBreak (Variables|Default|Getsa_empty) :!label _label_2)
                (:LoopBody
                  (if _array_element_2
                    (Utilities|Array|SetArrayElem (Variables|Default|Getsounding_ants) _array_index ant)
                    (Utilities|Array|SetArrayElem (Variables|Default|Getsa_empty) _array_index false)
                    (Utilities|Array|SetArrayElem (Variables|Default|Getsa_grunt_wait_ctr) _array_index 0.0)
                    (Utilities|Array|SetArrayElem (Variables|Default|Getsa_playing_grunt) _array_index false)
                    (Audio|Components|Audio|Play (Utilities|Array|Get(acopy) (Variables|Default|Getsa_footsteps) _array_index) 0.0)
                    (Transformation|SetWorldLocation (Utilities|Array|Get(acopy) (Variables|Default|Getsa_footsteps) _array_index) (Transformation|GetActorLocation ant) false false)
                    (goto _label_2 Break)))))))))))

(fn Remove
  (params (ant :type BP%20Ant%20AI%20Object%20Reference))
  (bind (_array_element _array_index) (Utilities|Array|ForEachLoopwithBreak (Variables|Default|Getsounding_ants) :!label _label)
    (:LoopBody
      (if (not (Utilities|Array|Get(acopy) (Variables|Default|Getsa_empty) _array_index))
        (if (== ant _array_element)
          (Utilities|Array|SetArrayElem (Variables|Default|Getsa_empty) _array_index true)
          (Audio|Components|Audio|Stop (Utilities|Array|Get(acopy) (Variables|Default|Getsa_footsteps) _array_index))
          (Math|Integer|DecrementInt (Variables|Default|Getassigned_ct)
            (:%20%20
              (goto _label Break))))))))

(fn AddFootstep
  (params (footstep :type Audio%20Component%20Object%20Reference))
  (Utilities|Array|AddUnique (Variables|Default|Getsa_footsteps) footstep))

(fn AddGrunt
  (params (grunt :type Audio%20Component%20Object%20Reference))
  (Utilities|Array|Add (Variables|Default|Getsa_grunts) grunt))