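; BP_FadeActor is a plane actor that fades out and destroys itself shortly after spawning.
; BeginPlay creates a dynamic material instance on the Plane, waits briefly, then starts fading.
; Tick drives the material's Opacity parameter down linearly over FadeTime and destroys the actor once that time elapses.
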(event EventBeginPlay
  (bind _plane (Variables|Default|GetPlane))
  (bind _returnvalue (Rendering|Material|CreateDynamicMaterialInstance _plane 0 (Rendering|Material|GetMaterial _plane 0) "None" :!class /Script/Engine.PrimitiveComponent))
  (Variables|Default|Setmat _returnvalue)
  (Utilities|FlowControl|Delay 0.5)
  (Variables|Default|Setfading true))

(event Collision|EventActorBeginOverlap
  (params (OtherActor :type Actor%20Object%20Reference)))

(event EventTick
  (params (DeltaSeconds :type Float%20%28single-precision%29))
  (if (Variables|Default|Getfading)
    (Variables|Default|Setfade_ctr (+ (Variables|Default|Getfade_ctr) DeltaSeconds))
    (if (> (Variables|Default|Getfade_ctr) (Variables|Default|Getfade_time))
      (Actor|DestroyActor)
      (else
        (Rendering|Material|SetScalarParameterValue (Variables|Default|Getmat) "Opacity" (- 1.0 (/ (Variables|Default|Getfade_ctr) (Variables|Default|Getfade_time))) :!class /Script/Engine.MaterialInstanceDynamic)))))

(fn ConstructionScript)