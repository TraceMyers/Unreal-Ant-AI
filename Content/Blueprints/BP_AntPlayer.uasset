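; BP_AntPlayer is the player ant Blueprint, and its graph handles music, ambience and nearby ant sounds.
; On begin play it attaches wind and intro song sounds, then starts the song loop after a fixed delay.
; SoundBox overlaps toggle footsteps and grunting on BP_AntAI actors.
; A counter limits new activations against MaxNearbyAnts, but every exiting ant decrements it, including ones never activated.
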(event OnComponentBeginOverlap(SoundBox)
  (params (OverlappedComponent :type Primitive%20Component%20Object%20Reference) (OtherActor :type Actor%20Object%20Reference) (OtherComp :type Primitive%20Component%20Object%20Reference) (OtherBodyIndex :type Integer) (bFromSweep :type Boolean) (SweepResult :type Hit%20Result%20Structure%20%28by%20ref%29))
  (if (<= (Variables|Default|Getsounding_ants_ct) (Variables|Default|Getmax_nearby_ants))
    (bind _asbp_ant_ai (Utilities|Casting|CastToBP_AntAI OtherActor))
    (Audio|Components|Audio|Play (Variables|/Game/Blueprints/BP_AntAI.BP_AntAI_C|GetFootsteps _asbp_ant_ai) 0.0)
    (Variables|/Game/Blueprints/BP_AntAI.BP_AntAI_C|Setgrunting _asbp_ant_ai true)
    (Math|Integer|IncrementInt (Variables|Default|Getsounding_ants_ct))))

(event OnComponentEndOverlap(SoundBox)
  (params (OverlappedComponent :type Primitive%20Component%20Object%20Reference) (OtherActor :type Actor%20Object%20Reference) (OtherComp :type Primitive%20Component%20Object%20Reference) (OtherBodyIndex :type Integer))
  (bind _asbp_ant_ai (Utilities|Casting|CastToBP_AntAI OtherActor))
  (Audio|Components|Audio|Stop (Variables|/Game/Blueprints/BP_AntAI.BP_AntAI_C|GetFootsteps _asbp_ant_ai))
  (Variables|/Game/Blueprints/BP_AntAI.BP_AntAI_C|Setgrunting _asbp_ant_ai false)
  (Math|Integer|DecrementInt (Variables|Default|Getsounding_ants_ct)))

(event EventBeginPlay
  (bind _rootcomponent (Variables|Transformation|GetRootComponent))
  (bind _song_loop (Variables|Default|Getsong_loop))
  (Audio|SpawnSoundAttached "/Game/sounds/wind_edited.wind_edited" _rootcomponent "None" "0, 0, 0" "0, 0, 0" "KeepRelativeOffset" false 1.0 1.0 0.0 0 0)
  (bind _returnvalue (Audio|SpawnSoundAttached "/Game/sounds/song_start.song_start" _rootcomponent "None" "0, 0, 0" "0, 0, 0" "KeepRelativeOffset" false 1.0 1.0 0.0 0 0))
  (Variables|Default|Setsong_start_ref _returnvalue)
  (Audio|Components|Audio|Stop _song_loop)
  (Utilities|FlowControl|Delay 86.0)
  (Audio|Components|Audio|Play _song_loop 0.0))

(event Collision|EventActorBeginOverlap
  (params (OtherActor :type Actor%20Object%20Reference)))

(event EventTick
  (params (DeltaSeconds :type Float%20%28single-precision%29)))

(fn ConstructionScript
  (|CallParentFunction))