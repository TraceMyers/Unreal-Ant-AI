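; BP_AntAI is an ant Blueprint that, in this graph, handles only intermittent grunt audio.
; BeginPlay silences the Footsteps and Grunt audio and picks a random first wait.
; While Grunting is set, Tick counters alternate between waiting and playing the Grunt sound from a random start offset for a set duration, re-randomizing each wait.
; Nothing here sets Grunting or restarts Footsteps.
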(event EventBeginPlay
  (Audio|Components|Audio|Stop (Variables|Default|GetFootsteps))
  (Audio|Components|Audio|Stop (Variables|Default|GetGrunt))
  (Variables|Default|SetGRUNT_WAIT (+ (* (Math|Random|RandomFloat) 15.0) 2.0)))

(event Collision|EventActorBeginOverlap
  (params (OtherActor :type Actor%20Object%20Reference)))

(event EventTick
  (params (DeltaSeconds :type Float%20%28single-precision%29))
  (if (Variables|Default|Getgrunting)
    (if (Variables|Default|Getplaying%20grunt)
      (bind _output_get (Variables|Default|Setgrunt_play_time (+ (Variables|Default|Getgrunt_play_time) DeltaSeconds)))
      (if (>= _output_get (Variables|Default|GetGRUNT_PLAY))
        (Audio|Components|Audio|Stop (Variables|Default|GetGrunt))
        (Variables|Default|Setplaying%20grunt false))
      (else
        (bind _output_get_2 (Variables|Default|Setgrunt_wait_ctr (+ (Variables|Default|Getgrunt_wait_ctr) DeltaSeconds)))
        (if (>= _output_get_2 (Variables|Default|GetGRUNT_WAIT))
          (Audio|Components|Audio|Play (Variables|Default|GetGrunt) (* (Math|Random|RandomFloat) 1e+01))
          (Variables|Default|SetGRUNT_WAIT (+ (* (Math|Random|RandomFloat) 15.0) 5.0))
          (Variables|Default|Setplaying%20grunt true)
          (Variables|Default|Setgrunt_play_time 0.0)
          (Variables|Default|Setgrunt_wait_ctr 0.0))))))

(fn ConstructionScript)